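; Health component shared by AI and player, tracking current and max health and mirroring them to UI.
; One tick after BeginPlay, it casts its owner to BP_AI to pick the enemy bar, otherwise the player HUD.
; DecreaseHealth updates that bar, adding text and a fresh-death result only for players.
; Both increase functions write only to the player HUD; IncreaseMaxHealth derives the maximum from current health plus the increment.
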(event EventBeginPlay
  (Utilities|FlowControl|DelayUntilNextTick)
  (bind _asbp_ai (Utilities|Casting|CastToBP_AI (Components|GetOwner))
    (:then
      (Variables|Default|SetHealth%20Bar%20Enemy%20Widget (Variables|/Game/AI/BP_AI.BP_AI_C|GetHealth%20Bar%20UI _asbp_ai))
      (Variables|Default|SetIsPlayer false))
    (:CastFailed
      (bind _asbp_third_person_character (Utilities|Casting|CastToBP_ThirdPersonCharacter (Game|GetPlayerCharacter 0)))
      (Variables|Default|SetHealth%20Bar%20Widget (Variables|/Game/ThirdPerson/Blueprints/BP_ThirdPersonCharacter.BP_ThirdPersonCharacter_C|GetHUD%20Widget _asbp_third_person_character))
      (Variables|Default|SetIsPlayer true)))
  (Progress|SetPercent (select (Variables|Default|GetIsPlayer) (Variables|/Game/UI/HUD/WD_HUD.WD_HUD_C|GetHealthBar (Variables|Default|GetHealth%20Bar%20Widget)) (Variables|/Game/UI/HUD/WD_HUD_Enemy.WD_HUD_Enemy_C|GetHealthBar (Variables|Default|GetHealth%20Bar%20Enemy%20Widget))) (/ (Variables|Health|GetCurrent%20Health) (Variables|Health|GetMax%20Health)))
  (if (Variables|Default|GetIsPlayer)
    (Rendering|Components|TextRender|SetText (Variables|/Game/UI/HUD/WD_HUD.WD_HUD_C|GetHealthText (Variables|Default|GetHealth%20Bar%20Widget)) (Utilities|Text|ToText(Float) (Variables|Health|GetCurrent%20Health) "HalfToEven"))))

(fn DecreaseHealth
  (params (Damage :type Float%20%28double-precision%29))
  (bind _isplayer (Variables|Default|GetIsPlayer))
  (if (not (<= (Variables|Health|GetCurrent%20Health) 0.0))
    (bind _output_get (Variables|Health|SetCurrent%20Health (- (Variables|Health|GetCurrent%20Health) Damage)))
    (Progress|SetPercent (select (Variables|Default|GetIsPlayer) (Variables|/Game/UI/HUD/WD_HUD.WD_HUD_C|GetHealthBar (Variables|Default|GetHealth%20Bar%20Widget)) (Variables|/Game/UI/HUD/WD_HUD_Enemy.WD_HUD_Enemy_C|GetHealthBar (Variables|Default|GetHealth%20Bar%20Enemy%20Widget))) (/ _output_get (Variables|Health|GetMax%20Health)))
    (if _isplayer
      (Rendering|Components|TextRender|SetText (select _isplayer (Variables|/Game/UI/HUD/WD_HUD.WD_HUD_C|GetHealthText (Variables|Default|GetHealth%20Bar%20Widget)) 0) (Utilities|Text|ToText(Float) (Variables|Health|GetCurrent%20Health) "HalfToEven"))
      (if (<= (Variables|Health|GetCurrent%20Health) 0.0)
        (return true)
        (else
          (return false))))
    (else
      (return true))))

(fn IncreaseMaxHealth
  (params (Incrementation :type Float%20%28double-precision%29))
  (bind _player_character_bp (Variables|Default|GetPlayer%20Character%20BP))
  (bind _hud_widget (Variables|/Game/ThirdPerson/Blueprints/BP_ThirdPersonCharacter.BP_ThirdPersonCharacter_C|GetHUD%20Widget _player_character_bp))
  (Variables|Health|SetMax%20Health (+ (Variables|Health|GetCurrent%20Health) Incrementation))
  (Progress|SetPercent (Variables|/Game/UI/HUD/WD_HUD.WD_HUD_C|GetHealthBar _hud_widget) (/ (Variables|Health|GetCurrent%20Health) (Variables|Health|GetMax%20Health)))
  (Rendering|Components|TextRender|SetText (Variables|/Game/UI/HUD/WD_HUD.WD_HUD_C|GetHealthText _hud_widget) (Utilities|Text|ToText(Float) (Variables|Health|GetCurrent%20Health) "HalfToEven")))

(fn IncreaseHealth
  (params (Added%20Health :type Float%20%28double-precision%29))
  (bind _player_character_bp (Variables|Default|GetPlayer%20Character%20BP))
  (bind _hud_widget (Variables|/Game/ThirdPerson/Blueprints/BP_ThirdPersonCharacter.BP_ThirdPersonCharacter_C|GetHUD%20Widget _player_character_bp))
  (Variables|Health|SetCurrent%20Health (+ (Variables|Health|GetCurrent%20Health) Added%20Health))
  (if (> (Variables|Health|GetCurrent%20Health) (Variables|Health|GetMax%20Health))
    (Variables|Health|SetCurrent%20Health (Variables|Health|GetMax%20Health)))
  (Progress|SetPercent (Variables|/Game/UI/HUD/WD_HUD.WD_HUD_C|GetHealthBar _hud_widget) (/ (Variables|Health|GetCurrent%20Health) (Variables|Health|GetMax%20Health)))
  (Rendering|Components|TextRender|SetText (Variables|/Game/UI/HUD/WD_HUD.WD_HUD_C|GetHealthText _hud_widget) (Utilities|Text|ToText(Float) (Variables|Health|GetCurrent%20Health) "HalfToEven")))