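; BP_InteractableActor is an interactable actor that shows an instruction widget while the player is inside its box trigger.
; Overlap identifies the player through the IsPlayerMessage call, lazily creates the WD_Instruction widget, and toggles viewport display and input on enter and exit.
; Pressing IA_Interact plays a click sound, hides the prompt and sets the Interacting flag, which releasing clears; the interaction itself only prints a debug string.
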(event OnComponentBeginOverlap(Box)
  (params (OverlappedComponent :type Primitive%20Component%20Object%20Reference) (OtherActor :type Actor%20Object%20Reference) (OtherComp :type Primitive%20Component%20Object%20Reference) (OtherBodyIndex :type Integer) (bFromSweep :type Boolean) (SweepResult :type Hit%20Result%20Structure%20%28by%20ref%29))
  ;[0.958 0.4223 1] Widget "[F] Grab the box" - When you enter the box it shows the widget and when you go out of the box it disappears
  (bind _yes_no_ (Class|BPICharacterInterface|IsPlayer?(Message) OtherActor))
  (if _yes_no_
    (Variables|Default|SetInteractingActor OtherActor)
    (Variables|Default|GetWDInstruction]
      (:then
        _)
      (:else
        (bind _returnvalue (UserInterface|CreateWidget "/Game/UI/WD_Instruction.WD_Instruction_C"))
        (Variables|Default|SetWDInstruction] _returnvalue)))
    (UserInterface|Viewport|AddtoViewport (Variables|Default|GetWDInstruction]) 0)
    (Input|EnableInput (Game|GetPlayerController 0))))

(event OnComponentEndOverlap(Box)
  (params (OverlappedComponent :type Primitive%20Component%20Object%20Reference) (OtherActor :type Actor%20Object%20Reference) (OtherComp :type Primitive%20Component%20Object%20Reference) (OtherBodyIndex :type Integer))
  ;[0.958 0.4223 1] Widget "[F] Grab the box" - When you enter the box it shows the widget and when you go out of the box it disappears
  (bind _yes_no_ (Class|BPICharacterInterface|IsPlayer?(Message) OtherActor))
  (if _yes_no_
    (Utilities|HideInstruction)
    (Input|DisableInput (Game|GetPlayerController 0))))

(event Custom|Start%20Interaction
  (params (InteractingActor :type Actor%20Object%20Reference))
  (Variables|Default|SetInteractingActor InteractingActor)
  (Variables|Default|SetInteracting true)
  (Utilities|HideInstruction)
  (Development|PrintString "Interacting" true true "(R=0.000000,G=0.660000,B=1.000000,A=1.000000)" 1e+01))

(event Custom|End%20Interaction
  (Variables|Default|SetInteracting false))

(event Input|EnhancedActionEvents|EnhancedInputActionIA_Interact
  (params (ActionValue :type Boolean) (ElapsedSeconds :type Float%20%28double-precision%29) (TriggeredSeconds :type Float%20%28double-precision%29) (InputAction :type Input%20Action%20Object%20Reference :default "/Game/ThirdPerson/Input/Actions/IA_Interact.IA_Interact"))
  (:Started
    (Audio|PlaySound2D "/Engine/VREditor/Sounds/UI/Gizmo_Handle_Clicked.Gizmo_Handle_Clicked" 1.0 1.0 0.0 0 0)
    (CallFunction|StartInteraction (Variables|Default|GetInteractingActor)))
  (:Completed
    (CallFunction|EndInteraction)))

(fn ConstructionScript)