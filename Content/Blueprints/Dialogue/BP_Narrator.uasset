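; BP_Narrator is a trigger-zone narrator that shows a dialogue line on screen with a sound when the player overlaps it.
; Talk advances TalkIndex and, only while no valid UI exists, creates the widget, then after a delay sets its text from the Dialogue array.
; Leaving the zone removes the widget after a longer delay.
; The index bounds check is unconnected, so Talk's removal branch never runs.
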(event OnComponentBeginOverlap(TriggerZone)
  (params (OverlappedComponent :type Primitive%20Component%20Object%20Reference) (OtherActor :type Actor%20Object%20Reference) (OtherComp :type Primitive%20Component%20Object%20Reference) (OtherBodyIndex :type Integer) (bFromSweep :type Boolean) (SweepResult :type Hit%20Result%20Structure%20%28by%20ref%29))
  (bind _yes_no_ (Class|BPICharacterInterface|IsPlayer?(Message) OtherActor))
  (if _yes_no_
    (CallFunction|Talk)))

(event OnComponentEndOverlap(TriggerZone)
  (params (OverlappedComponent :type Primitive%20Component%20Object%20Reference) (OtherActor :type Actor%20Object%20Reference) (OtherComp :type Primitive%20Component%20Object%20Reference) (OtherBodyIndex :type Integer))
  (bind _yes_no_ (Class|BPICharacterInterface|IsPlayer?(Message) OtherActor))
  (if _yes_no_
    (Utilities|FlowControl|Delay 1e+01)
    (Widget|RemovefromParent (Variables|Default|GetUI))))

(event EventTalk
  (Math|Integer|IncrementInt (Variables|Default|GetTalkIndex)
    (:%20%20
      (if true
        (Variables|Default|GetUI
          (:then)
          (:else
            (bind _returnvalue (UserInterface|CreateWidget "/Game/Blueprints/Dialogue/WD_Dialogue.WD_Dialogue_C" (Game|GetPlayerController 0)))
            (bind _output_get (Variables|Default|SetUI _returnvalue))
            (UserInterface|Viewport|AddtoViewport _output_get 0)
            (Utilities|FlowControl|Delay 5.0)
            (Rendering|Components|TextRender|SetText (Variables|/Game/Blueprints/Dialogue/WD_Dialogue.WD_Dialogue_C|GetTalkText (Variables|Default|GetUI)) (Utilities|Text|ToText(String) (Utilities|Array|Get(acopy) (Variables|Default|GetDialogue) (Variables|Default|GetTalkIndex))))
            (Audio|PlaySound2D 0 1.0 1.0 0.0 0 0)))
        (else
          (Widget|RemovefromParent (Variables|Default|GetUI)))))))

(fn ConstructionScript)