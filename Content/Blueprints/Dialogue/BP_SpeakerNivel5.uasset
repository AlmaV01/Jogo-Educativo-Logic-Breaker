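; BP_SpeakerNivel5 is an interactable speaker that plays a timed sequence of dialogue lines on screen.
; When interaction starts and the parent logic leaves it active, it resets the line index and creates a WD_Dialogue widget for the first player controller.
; A delay-driven loop shows each Dialogue entry in turn, removing the widget immediately after setting the last line.
; Ending interaction only calls the parent, so it does not stop the sequence.
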(event EventStartInteraction
  (params (InteractingActor :type Actor%20Object%20Reference))
  (|CallParentFunction InteractingActor)
  (if (Variables|Default|GetInteracting)
    (Variables|Default|SetTalkIndex 0)
    (CallFunction|Talk)))

(event EventEndInteraction
  (|CallParentFunction))

(event EventTalk
  (bind _returnvalue (UserInterface|CreateWidget "/Game/Blueprints/Dialogue/WD_Dialogue.WD_Dialogue_C" (Game|GetPlayerController 0)))
  (bind _output_get (Variables|Default|SetUI _returnvalue))
  (UserInterface|Viewport|AddtoViewport _output_get 0)
  (Rendering|Components|TextRender|SetText (Variables|/Game/Blueprints/Dialogue/WD_Dialogue.WD_Dialogue_C|GetTalkText (Variables|Default|GetUI)) (Utilities|Text|ToText(String) (Utilities|Array|Get(acopy) (Variables|Default|GetDialogue) (Variables|Default|GetTalkIndex))) :!label _label)
  (Math|Integer|IncrementInt (Variables|Default|GetTalkIndex)
    (:%20%20
      (if (< (Variables|Default|GetTalkIndex) (Utilities|Array|Length (Variables|Default|GetDialogue)))
        (Utilities|FlowControl|Delay 2.0)
        (goto _label)
        (else
          (Widget|RemovefromParent (Variables|Default|GetUI)))))))

(fn ConstructionScript
  (|CallParentFunction))