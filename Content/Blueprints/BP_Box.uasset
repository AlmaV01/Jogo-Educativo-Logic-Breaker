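; BP_Box is an interactable box that a Character can pick up, carry and set down.
; Starting interaction plays a carrying montage on the character, attaches the box to the left-hand socket and eases it into place with MoveComponentTo.
; Ending interaction stops the montage and traces downward ahead of the character; on a hit, the box detaches and eases to that point.
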(event Custom|DropBox
  (bind _character (Variables|Default|GetCharacter))
  (bind _returnvalue (Transformation|GetActorForwardVector _character))
  (bind _returnvalue_2 (Transformation|GetActorLocation _character))
  (bind _returnvalue_3 (* _returnvalue 1e+02))
  (bind _returnvalue_4 (+ _returnvalue_2 _returnvalue_3))
  (bind (_outhit _returnvalue_5) (Collision|LineTraceByChannel _returnvalue_4 (+ _returnvalue_4 "0.000000,0.000000,-500.000000") "TraceTypeQuery1" false 0 "ForDuration"))
  (if _returnvalue_5
    (Transformation|DetachFromActor "KeepWorld" "KeepWorld" "KeepWorld")
    (Components|MoveComponentTo (Variables|Default|GetDefaultSceneRoot) (.Location (Collision|BreakHitResult _outhit)) (Math|Rotator|MakeRotator 0.0 0.0 (.yaw (Transformation|GetActorRotation))) true true 0.3 false)))

(event EventStartInteraction
  (params (InteractingActor :type Actor%20Object%20Reference))
  (|CallParentFunction InteractingActor)
  (bind _ascharacter (Utilities|Casting|CastToCharacter (Variables|Default|GetInteractingActor)))
  (Variables|Default|SetCharacter _ascharacter)
  (Animation|Montage|PlayMontage (Variables|/Script/Engine.Character|GetMesh _ascharacter) "/Game/Characters/RPG_Character/Animations/Locomotion/Carrying_Montage.Carrying_Montage"
    (:then
      (Transformation|AttachComponentToComponent (Variables|/Script/Engine.Character|GetMesh _ascharacter) "hand_lSocket" "KeepWorld" "KeepWorld" "KeepWorld" true)
      (Components|MoveComponentTo (Variables|Default|GetDefaultSceneRoot) "0, 0, 0" "0, 0, 0" true true 0.3 true))))

(fn ConstructionScript
  (|CallParentFunction))

(fn EndInteraction
  (bind _character (Variables|Default|GetCharacter)
    (:then
      (Animation|StopAnimMontage _character "/Game/Characters/RPG_Character/Animations/Locomotion/Carrying_Montage.Carrying_Montage")
      (CallFunction|DropBox)
      (return))
    (:else)))