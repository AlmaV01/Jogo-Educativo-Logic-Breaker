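; BP_ANDGate is a puzzle logic gate that powers its linked cable only when two inputs are on.
; Poweron and PowerOff events raise and lower a shared PowerCount instead of tracking individual sources.
; Reaching exactly two sets IsFilling on LinkedCable, and dropping below two clears it, provided the cable reference is valid.
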(event EventPoweron
  (bind _linkedcable (Variables|Default|GetLinkedCable))
  ;[1 1 1] AND Logic
  (bind _output_get (Variables|Default|SetPowerCount (+ (Variables|Default|GetPowerCount) 1)))
  (if (== _output_get 2)
    ;[1 1 1] Or Logic
    (Utilities|IsValid _linkedcable
      (:Is%20Valid
        (Variables|/Game/Blueprints/Puzzle/BP_Cable.BP_Cable_C|SetIsFilling? _linkedcable true)))))

(event EventPowerOff
  (bind _linkedcable (Variables|Default|GetLinkedCable))
  ;[1 1 1] AND Logic
  (bind _output_get (Variables|Default|SetPowerCount (- (Variables|Default|GetPowerCount) 1)))
  (if (< _output_get 2)
    ;[1 1 1] Or Logic
    (Utilities|IsValid _linkedcable
      (:Is%20Valid
        (Variables|/Game/Blueprints/Puzzle/BP_Cable.BP_Cable_C|SetIsFilling? _linkedcable false)))))

(fn ConstructionScript)