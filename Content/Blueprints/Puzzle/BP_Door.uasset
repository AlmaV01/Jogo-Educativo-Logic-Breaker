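; Puzzle door Blueprint with four panels that slide apart when powered on and close when powered off.
; Poweron plays an opening sound and runs a Timeline that linearly eases the left, right, top and bottom panels outward through relative locations.
; PowerOff plays a closing sound and reverses the same Timeline.
; A second Timeline with closing offsets is left unconnected and never runs.
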(event EventPoweron
  ;[1 1 1] Open the door
  (Audio|PlaySound2D "/Game/Audio/Sounds/opening_door.opening_door" 1.0 1.0 0.0 0 0)
  (bind _alpha (Timeline|Timeline Play)
    (:Update
      (Utilities|FlowControl|Sequence
        (:then_0
          (Transformation|SetRelativeLocation (Variables|Default|Getleft_door) (Math|Interpolation|Ease :Function "Linear" :Alpha _alpha :B "-70.000000,0.000000,0.000000") false false)
          (Transformation|SetRelativeLocation (Variables|Default|Gettop_door) (Math|Interpolation|Ease :Function "Linear" :Alpha _alpha :B "0.000000,0.000000,90.000000") false false))
        (:then_1
          (Transformation|SetRelativeLocation (Variables|Default|Getright_door) (Math|Interpolation|Ease :Function "Linear" :Alpha _alpha :B "70.000000,0.000000,0.000000") false false)
          (Transformation|SetRelativeLocation (Variables|Default|Getbottom_door) (Math|Interpolation|Ease :Function "Linear" :Alpha _alpha :B "0.000000,0.000000,-203.000000") false false))))))

(event EventPowerOff
  ;[1 1 1] Close the door[
  (Audio|PlaySound2D "/Game/Audio/Sounds/closing_door.closing_door" 1.0 1.0 0.0 0 0)
  ;[1 1 1] Open the door
  (bind _alpha (Timeline|Timeline Reverse)
    (:Update
      (Utilities|FlowControl|Sequence
        (:then_0
          (Transformation|SetRelativeLocation (Variables|Default|Getleft_door) (Math|Interpolation|Ease :Function "Linear" :Alpha _alpha :B "-70.000000,0.000000,0.000000") false false)
          (Transformation|SetRelativeLocation (Variables|Default|Gettop_door) (Math|Interpolation|Ease :Function "Linear" :Alpha _alpha :B "0.000000,0.000000,90.000000") false false))
        (:then_1
          (Transformation|SetRelativeLocation (Variables|Default|Getright_door) (Math|Interpolation|Ease :Function "Linear" :Alpha _alpha :B "70.000000,0.000000,0.000000") false false)
          (Transformation|SetRelativeLocation (Variables|Default|Getbottom_door) (Math|Interpolation|Ease :Function "Linear" :Alpha _alpha :B "0.000000,0.000000,-203.000000") false false))))))

(fn ConstructionScript)