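; BP_NOTGate is a puzzle logic gate that inverts the power signal it receives.
; Poweron clears IsPowered and stops LinkedCable filling, while PowerOff sets IsPowered and starts the cable filling.
; BeginPlay calls PowerOff, so the gate outputs power until it is switched on.
; Disconnected AND-style PowerCount nodes remain in the graph but never run.
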(event EventBeginPlay
  ;[1 1 1] NOT Logic
  (Variables|Default|SetIsPowered? true)
  (CallFunction|PowerOff))

(event EventPoweron
  (bind _linkedcable (Variables|Default|GetLinkedCable))
  ;[1 1 1] NOT Logic
  (Variables|Default|SetIsPowered? false)
  ;[1 1 1] Or Logic
  (Utilities|IsValid _linkedcable
    (:Is%20Valid
      (Variables|/Game/Blueprints/Puzzle/BP_Cable.BP_Cable_C|SetIsFilling? _linkedcable false))))

(event EventPowerOff
  (bind _linkedcable (Variables|Default|GetLinkedCable))
  ;[1 1 1] NOT Logic
  (Variables|Default|SetIsPowered? true)
  ;[1 1 1] Or Logic
  (Utilities|IsValid _linkedcable
    (:Is%20Valid
      (Variables|/Game/Blueprints/Puzzle/BP_Cable.BP_Cable_C|SetIsFilling? _linkedcable true))))

(fn ConstructionScript)