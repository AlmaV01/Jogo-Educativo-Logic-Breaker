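; Puzzle pressure plate that activates while the third-person character, a BP_Box or a CuboAzulPresion overlaps its trigger box.
; An overlap counter keeps it active until the last valid actor leaves.
; Activate and Deactivate play a sound, swap the frame material and drive a Timeline that lowers or raises the button.
; A valid LinkedCable has its IsFilling flag set to match the plate state.
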(event OnComponentBeginOverlap(Box)
  (params (OverlappedComponent :type Primitive%20Component%20Object%20Reference) (OtherActor :type Actor%20Object%20Reference) (OtherComp :type Primitive%20Component%20Object%20Reference) (OtherBodyIndex :type Integer) (bFromSweep :type Boolean) (SweepResult :type Hit%20Result%20Structure%20%28by%20ref%29))
  (bind _linkedcable (Variables|Default|GetLinkedCable))
  (Utilities|Casting|CastToBP_ThirdPersonCharacter OtherActor
    (:then
      _)
    (:CastFailed
      (Utilities|Casting|CastToBP_Box OtherActor
        (:then
          _)
        (:CastFailed
          (Utilities|Casting|CastToCuboAzulPresion OtherActor)))))
  (CallFunction|Activate)
  (Math|Integer|IncrementInt (Variables|Default|GetOverlappedActors)
    (:%20%20
      (Utilities|IsValid _linkedcable
        (:Is%20Valid
          (Variables|/Game/Blueprints/Puzzle/BP_Cable.BP_Cable_C|SetIsFilling? _linkedcable true))))))

(event OnComponentEndOverlap(Box)
  (params (OverlappedComponent :type Primitive%20Component%20Object%20Reference) (OtherActor :type Actor%20Object%20Reference) (OtherComp :type Primitive%20Component%20Object%20Reference) (OtherBodyIndex :type Integer))
  (bind _linkedcable (Variables|Default|GetLinkedCable))
  (Utilities|Casting|CastToBP_ThirdPersonCharacter OtherActor
    (:then
      _)
    (:CastFailed
      (Utilities|Casting|CastToBP_Box OtherActor
        (:then
          _)
        (:CastFailed
          (Utilities|Casting|CastToCuboAzulPresion OtherActor)))))
  (bind _result (Math|Integer|DecrementInt (Variables|Default|GetOverlappedActors))
    (:%20%20
      (if (== _result 0)
        (CallFunction|Deactivate)
        (Utilities|IsValid _linkedcable
          (:Is%20Valid
            (Variables|/Game/Blueprints/Puzzle/BP_Cable.BP_Cable_C|SetIsFilling? _linkedcable false)))))))

(event Custom|Activate
  ;[1 1 1] Boton Activo
  (if (not (Variables|Default|GetIsActive))
    (Audio|PlaySoundatLocation "/Engine/VREditor/Sounds/UI/Click_on_Button.Click_on_Button" (Transformation|GetActorLocation) "0, 0, 0" 1.0 1.0 0.0 0 0 0 0)
    (Variables|Default|SetIsActive true)
    (Rendering|Material|SetMaterial (Variables|Default|GetFrame) 0 "/Game/Blueprints/Puzzle/Materials/MAT_PlateFrameActive.MAT_PlateFrameActive")
    ;[1 0.4991 0.8748] Animación
    (bind _alpha (Timeline|Timeline Play)
      (:Update
        (Transformation|SetRelativeLocation (Variables|Default|GetButton) (Math|Vector|MakeVector 0.0 0.0 (Math|Interpolation|Ease "Linear" _alpha (Math|Float|MakeLiteralFloat 0.0) (Math|Float|MakeLiteralFloat -4.0))) false false)))))

(event Custom|Deactivate
  ;[1 1 1] Boton Inactivo
  (if (Variables|Default|GetIsActive)
    (Audio|PlaySoundatLocation "/Engine/VREditor/Sounds/UI/Camera_Shutter.Camera_Shutter" (Transformation|GetActorLocation) "0, 0, 0" 1.0 1.0 0.0 0 0 0 0)
    (Variables|Default|SetIsActive false)
    (Rendering|Material|SetMaterial (Variables|Default|GetFrame) 0 "/Game/LevelPrototyping/Materials/MI_PrototypeGrid_Blue.MI_PrototypeGrid_Blue")
    ;[1 0.4991 0.8748] Animación
    (bind _alpha (Timeline|Timeline ReverseFromEnd)
      (:Update
        (Transformation|SetRelativeLocation (Variables|Default|GetButton) (Math|Vector|MakeVector 0.0 0.0 (Math|Interpolation|Ease "Linear" _alpha (Math|Float|MakeLiteralFloat 0.0) (Math|Float|MakeLiteralFloat -4.0))) false false)))))

(fn ConstructionScript)