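; BP_AI is an enemy character with a health component, an overhead health bar that turns toward the player camera each tick, and an Attack montage.
; Damage plays a random hit montage, launches it along the player's facing direction and reduces BPCHealth.
; When DecreaseHealth returns true, the mesh switches to physics simulation as a ragdoll.
; A separate Ragdoll event enables the same simulation after a short delay.
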(event Custom|Ragdoll
  ;[1 1 1] Ragdoll
  (Utilities|FlowControl|Delay 2.0)
  (Physics|SetSimulatePhysics (Variables|Character|GetMesh) true))

(event EventTick
  (params (DeltaSeconds :type Float%20%28single-precision%29))
  ;[1 1 1] Widget
  (Transformation|SetWorldRotation (Variables|Default|GetHealth%20Bar%20Widget) (Math|Rotator|FindLookatRotation (Transformation|GetWorldLocation (Variables|Default|GetHealth%20Bar%20Widget)) (Transformation|GetWorldLocation (Variables|/Script/Engine.PlayerCameraManager|GetTransformComponent (Game|GetPlayerCameraManager 0)))) false false))

(event Game|Damage|EventAnyDamage
  (params (Damage :type Float%20%28single-precision%29) (DamageType :type Damage%20Type%20Object%20Reference) (InstigatedBy :type Controller%20Object%20Reference) (DamageCauser :type Actor%20Object%20Reference))
  (Animation|PlayAnimMontage (Utilities|Array|Get(acopy) (Variables|Default|GetHitAnims) (Math|Random|RandomIntegerinRange 0 (- (Utilities|Array|Length (Variables|Default|GetHitAnims)) 1))) 1.0 "None")
  (bind _asbp_third_person_character (Utilities|Casting|CastToBP_ThirdPersonCharacter (Game|GetPlayerCharacter 0)))
  (Character|LaunchCharacter (* (Math|Vector|GetForwardVector (Transformation|GetActorRotation _asbp_third_person_character)) 7e+02) false false)
  (bind _isplayerdead_ (Default|DecreaseHealth (Variables|Default|GetBPC_Health) Damage))
  (if _isplayerdead_
    (Collision|SetCollisionObjectType (Variables|Character|GetMesh) "ECC_PhysicsBody")
    (Physics|SetSimulatePhysics (Variables|Character|GetMesh) true)))

(event EventBeginPlay
  (bind _returnvalue (UserInterface|CreateWidget "/Game/UI/HUD/WD_HUD_Enemy.WD_HUD_Enemy_C"))
  (bind _output_get (Variables|Default|SetHealth%20Bar%20UI _returnvalue))
  (UserInterface|SetWidget (Variables|Default|GetHealth%20Bar%20Widget) _output_get))

(fn ConstructionScript)

(fn Attack
  (Animation|PlayAnimMontage "/Game/Characters/RPG_Character/Animations/Attack/Anim_Attack01_Character.Anim_Attack01_Character" 1.0 "None")
  (return 0.0))