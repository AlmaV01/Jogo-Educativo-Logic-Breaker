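; Slime enemy that chases the player on sight and plays an attack when its Ataque trigger overlaps them.
; PawnSensing starts AIMoveTo, and a CanAttack flag gates attacks and halts movement, though the target reference is cleared before ApplyDamage.
; Taking damage plays a hit montage and sound, launches it along the player's facing and reduces BPCHealth.
; A health bar widget faces the camera, then hides on death before the mesh ragdolls.
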(event OnSeePawn(PawnSensing)
  (params (Pawn :type Pawn%20Object%20Reference))
  (Variables|Default|SetIsSeeingPlayer? true)
  (CallFunction|FollowPlayer)
  (Utilities|FlowControl|Delay 2.0))

(event OnComponentBeginOverlap(ataque)
  (params (OverlappedComponent :type Primitive%20Component%20Object%20Reference) (OtherActor :type Actor%20Object%20Reference) (OtherComp :type Primitive%20Component%20Object%20Reference) (OtherBodyIndex :type Integer) (bFromSweep :type Boolean) (SweepResult :type Hit%20Result%20Structure%20%28by%20ref%29))
  (bind _asbp_third_person_character (Utilities|Casting|CastToBP_ThirdPersonCharacter OtherActor))
  (Variables|Default|SetCharacter _asbp_third_person_character)
  (CallFunction|AttackPlayer))

(event Custom|Follow%20Player
  (Variables|Default|SetcanAttack? true)
  (if (Variables|Default|GetIsSeeingPlayer?)
    (AI|AIMoveTo self "0, 0, 0" (Game|GetPlayerCharacter 0) 7e+01 false)
    (else
      (Variables|Default|SetIsSeeingPlayer? false))))

(event Custom|Attack%20Player
  (if (Variables|Default|GetcanAttack?)
    (Variables|Default|SetcanAttack? false)
    (bind _returnvalue (Animation|PlayAnimMontage "/Game/Characters/ENEMIES/Slime/Anim_Attack01_Slime.Anim_Attack01_Slime" 1.0 "None"))
    (CallFunction|AttackPlayer)
    (Utilities|FlowControl|Delay _returnvalue)
    (Variables|Default|SetcanAttack? true)
    (bind _output_get (Variables|Default|SetCharacter 0))
    (Game|Damage|ApplyDamage _output_get 1e+01 0 0)))

(event EventBeginPlay
  (bind _returnvalue (UserInterface|CreateWidget "/Game/UI/HUD/WD_HUD_Enemy.WD_HUD_Enemy_C"))
  (bind _output_get (Variables|Default|SetHealth%20Bar%20UI _returnvalue))
  (UserInterface|SetWidget (Variables|Default|GetHealthBar) _output_get))

(event EventTick
  (params (DeltaSeconds :type Float%20%28single-precision%29))
  (Transformation|SetWorldRotation (Variables|Default|GetHealthBar) (Math|Rotator|FindLookatRotation (Transformation|GetWorldLocation (Variables|Default|GetHealthBar)) (Transformation|GetWorldLocation (Variables|/Script/Engine.PlayerCameraManager|GetTransformComponent (Game|GetPlayerCameraManager 0)))) false false)
  (Utilities|FlowControl|Delay 0.2)
  (if (not (Variables|Default|GetcanAttack?))
    (Components|Movement|StopMovementImmediately (Variables|Character|GetCharacterMovement))))

(event Game|Damage|EventAnyDamage
  (params (Damage :type Float%20%28single-precision%29) (DamageType :type Damage%20Type%20Object%20Reference) (InstigatedBy :type Controller%20Object%20Reference) (DamageCauser :type Actor%20Object%20Reference))
  (Animation|PlayAnimMontage "/Game/Characters/ENEMIES/Slime/Anim_Hit_Slime.Anim_Hit_Slime" 1.0 "None")
  (bind _asbp_third_person_character (Utilities|Casting|CastToBP_ThirdPersonCharacter (Game|GetPlayerCharacter 0)))
  (Character|LaunchCharacter (* (Math|Vector|GetForwardVector (Transformation|GetActorRotation _asbp_third_person_character)) 7e+02) false false)
  (Audio|PlaySoundatLocation 0 (Transformation|GetActorLocation) "0, 0, 0" 1.0 (Math|Random|RandomFloatinRange 1.0 1.3) 0.0 0 0 0 0)
  (bind _isplayerdead_ (Default|DecreaseHealth (Variables|Default|GetBPC_Health) Damage))
  (if _isplayerdead_
    (Utilities|FlowControl|Delay 0.2)
    (Animation|Montage|PlayMontage (Variables|Character|GetMesh) "/Game/Characters/ENEMIES/Slime/Anim_Slime_Die.Anim_Slime_Die"
      (:then
        (Rendering|SetVisibility (Variables|Default|GetHealthBar) false false)
        (Utilities|FlowControl|Delay 0.8)
        (Physics|SetSimulatePhysics (Variables|Character|GetMesh) true)))
    (else
      (Utilities|FlowControl|Delay 0.5))))

(fn ConstructionScript)